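; BP_ChessPlayer is the chess player Blueprint that selects the board tile under the mouse cursor.
; It shows the mouse cursor on BeginPlay, then updates the cursor location every Tick.
; Each update runs a complex Visibility trace under the cursor and stores any hit location.
; GridObject converts that location to a row and column and sets it as the selected tile, with no click needed.
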(event EventBeginPlay
  (Variables|/Script/Engine.PlayerController|SetbShowMouseCursor (Game|GetPlayerController 0) true))

(event Collision|EventActorBeginOverlap
  (params (OtherActor :type Actor%20Object%20Reference)))

(event EventTick
  (params (DeltaSeconds :type Float%20%28single-precision%29))
  (CallFunction|UpdateCursorLocation))

(fn ConstructionScript)

(fn UpdateCursorLocation
  (bind _returnvalue (Game|GetPlayerController 0))
  (bind _gridobject (Variables|Default|GetGridObject))
  (bind (_hitresult _returnvalue_2) (Game|Player|GetHitResultUnderCursorbyChannel _returnvalue "TraceTypeQuery1" true))
  (if _returnvalue_2
    (bind _output_get (LocalVariables|SetCursorLocation (.Location (Collision|BreakHitResult _hitresult))))
    (bind (_isvalid _row _column) (Default|LocationtoTile _gridobject _output_get))
    (Default|SetSelectedTile _gridobject _row _column)))